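; Player_1 is a player Blueprint that moves a physics-driven Cube and drops bombs, apparently for a bomb-placing game.
; Each tick it turns the Forwardback and LeftRight axis values into a horizontal force on the Cube, applied as an acceleration change.
; The Bomb input spawns a Bomb_1 above the Cube and increments Boms until it equals MaxBombs.
; Nothing in this Blueprint decrements that count.
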(event EventTick
  (params (DeltaSeconds :type Float%20%28single-precision%29))
  (Physics|AddForce (Variables|Default|GetCube) (Math|Vector|MakeVector (* (Input|AxisValues|GetForward/back) 1e+04) (* (Input|AxisValues|GetLeft/Right) 1e+04) 0.0) "None" true))

(event Input|ActionEvents|InputActionBomb
  (params (Key :type Key%20Structure))
  (bind _cube (Variables|Default|GetCube))
  (bind _returnvalue (Transformation|GetWorldLocation _cube))
  (:Pressed
    (if (!= (Variables|Default|GetBoms) (Variables|Default|GetMaxBombs))
      (Game|SpawnActorfromClass "/Game/blueprints/Assets/Bomb/Bomb_1.Bomb_1_C" (Math|Conversions|ToTransform(Vector) (Math|Vector|MakeVector (.x _returnvalue) (.y _returnvalue) (+ (.z _returnvalue) 2.5e+02))) "Undefined" 0 0)
      (Math|Integer|IncrementInt (Variables|Default|GetBoms)))))

(fn ConstructionScript)